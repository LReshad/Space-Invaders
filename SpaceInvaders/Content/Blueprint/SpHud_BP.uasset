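; SpHud_BP is a HUD Blueprint that shows the player's Life_Widget and handles its removal when lives run out.
; BeginPlay caches the game instance, adds the widget to the viewport, then caches the ship player controller and sets game-only input.
; The widget's owning-player reference is read before that controller is cached.
; Tick polls NoLife and, while true, removes the widget and shows the mouse cursor.
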(event EventBeginPlay
  (Utilities|FlowControl|Sequence
    (:then_0
      (bind _assp_game_instance_bp (Utilities|Casting|CastToSpGameInstance_BP (Game|GetGameInstance)))
      (Variables|Default|SetGameInstance _assp_game_instance_bp))
    (:then_1
      (bind _returnvalue (UserInterface|CreateWidget "/Game/Widget/Life_Widget.Life_Widget_C" (stale _output_get)))
      (UserInterface|Viewport|AddtoViewport _returnvalue 0))
    (:then_2
      (bind _asship_palyer_controller_bp (Utilities|Casting|CastToShipPalyerController_BP (Game|GetPlayerController 0)))
      (bind _output_get (Variables|Default|SetPlayerController _asship_palyer_controller_bp))
      (Input|SetInputModeGameOnly _output_get))))

(event Collision|EventActorBeginOverlap
  (params (OtherActor :type Actor%20Object%20Reference)))

(event EventTick
  (params (DeltaSeconds :type Float%20%28single-precision%29))
  (if (Variables|Default|GetbNoLife)
    (Widget|RemovefromParent (stale EventBeginPlay _returnvalue))
    (Variables|/Script/Engine.PlayerController|SetbShowMouseCursor (Variables|Default|GetPlayerController) true)))

(fn ConstructionScript)