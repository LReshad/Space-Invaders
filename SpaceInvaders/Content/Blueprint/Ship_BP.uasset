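; Player ship for a 2D Paper2D shooter that takes damage from alien projectiles and ends the game.
; Projectile hits reduce life stored in the game instance, then either flash an explosion flipbook or trigger game over.
; Tick also triggers game over at a fixed score.
; Both endings set the HUD's NoLife flag, show the GameOver widget and destroy the ship.
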(event OnComponentHit(Ship)
  (params (HitComponent :type Primitive%20Component%20Object%20Reference) (OtherActor :type Actor%20Object%20Reference) (OtherComp :type Primitive%20Component%20Object%20Reference) (NormalImpulse :type Vector :default "0, 0, 0") (Hit :type Hit%20Result%20Structure%20%28by%20ref%29))
  (Utilities|Casting|CastToAlienProjectile_BP OtherActor)
  (CallFunction|DecreseCurrentLife)
  (CallFunction|CheckLife))

(event Custom|checkLife
  (if (<= (Variables|/Game/Blueprint/SpGameInstance_BP.SpGameInstance_BP_C|GetCurrentLife (Variables|Default|GetGameInstance_BP)) 1.0)
    (Variables|/Game/Blueprint/SpHud_BP.SpHud_BP_C|SetbNoLife (Variables|Default|GetGameHud) true)
    (bind _returnvalue (UserInterface|CreateWidget "/Game/Widget/GameOver.GameOver_C"))
    (UserInterface|Viewport|AddtoViewport _returnvalue 0)
    (Actor|DestroyActor)
    (else
      (CallFunction|UpdateAnimation))))

(event Custom|UpdateAnimation
  (bind _ship (Variables|Default|GetShip))
  (Sprite|SetFlipbook _ship "/Game/FlipBook/ExplosionFlipBook.ExplosionFlipBook")
  (Utilities|FlowControl|Delay 0.3)
  (Sprite|SetFlipbook _ship "/Game/FlipBook/l0_SpaceShip.l0_SpaceShip"))

(event Collision|EventActorBeginOverlap
  (params (OtherActor :type Actor%20Object%20Reference)))

(event EventBeginPlay
  (bind _assp_game_instance_bp (Utilities|Casting|CastToSpGameInstance_BP (Game|GetGameInstance)))
  (Variables|Default|SetGameInstance_BP _assp_game_instance_bp)
  (bind _assp_hud_bp (Utilities|Casting|CastToSpHud_BP (HUD|GetHUD (Game|GetPlayerController 0))))
  (Variables|Default|SetGameHud _assp_hud_bp))

(event EventPlaySound
  (Audio|PlaySound2D "/Game/Assets/Sound/slimeball.slimeball" 0.75))

(event EventTick
  (params (DeltaSeconds :type Float%20%28single-precision%29))
  (if (== (Variables|/Game/Blueprint/SpGameInstance_BP.SpGameInstance_BP_C|GetScore (Variables|Default|GetGameInstance_BP)) 400)
    (Variables|/Game/Blueprint/SpHud_BP.SpHud_BP_C|SetbNoLife (Variables|Default|GetGameHud) true)
    (bind _returnvalue (UserInterface|CreateWidget "/Game/Widget/GameOver.GameOver_C"))
    (UserInterface|Viewport|AddtoViewport _returnvalue 0)
    (Actor|DestroyActor)))

(fn ConstructionScript)

(fn DecreseCurrentLife
  (bind _gameinstance_bp (Variables|Default|GetGameInstance_BP))
  (Variables|/Game/Blueprint/SpGameInstance_BP.SpGameInstance_BP_C|SetCurrentLife _gameinstance_bp (- (Variables|/Game/Blueprint/SpGameInstance_BP.SpGameInstance_BP_C|GetCurrentLife _gameinstance_bp) 33.33)))